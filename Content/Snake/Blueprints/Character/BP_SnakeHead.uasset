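; BP_SnakeHead is the player-controlled head of a Snake game, moving in fixed steps and growing when it eats food.
; Enhanced Input sets the direction and immediately moves one step, while a Delay in Tick repeats steps at intervals.
; Each move feeds a look-ahead position to the level's SnakeTrack actor, which updates body segments on timed steps.
; Overlapping BP_Food destroys it and adds a spawned BP_SnakeBody to that track.
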(event OnComponentBeginOverlap(Head)
  (params (OverlappedComponent :type Primitive%20Component%20Object%20Reference) (OtherActor :type Actor%20Object%20Reference) (OtherComp :type Primitive%20Component%20Object%20Reference) (OtherBodyIndex :type Integer) (bFromSweep :type Boolean) (SweepResult :type Hit%20Result%20Structure%20%28by%20ref%29))
  (bind _snaketrack (Variables|Default|GetSnakeTrack))
  (bind _asbp_food (Utilities|Casting|CastToBP_Food OtherActor))
  (Actor|DestroyActor _asbp_food)
  (bind _returnvalue (Game|SpawnActorfromClass "/Game/Snake/Blueprints/Character/BP_SnakeBody.BP_SnakeBody_C" (Transformation|GetActorTransform self) "AlwaysSpawn" "MultiplyWithRoot" 0 0))
  (Utilities|Array|Add (Variables|/Script/FeaturCollection.SnakeTrack|GetSnakeBodyActor _snaketrack) _returnvalue)
  (Class|SnakeTrack|SnakeBodyUpdate _snaketrack))

(event Input|EnhancedActionEvents|EnhancedInputActionIA_SnakeMove
  (params (ActionValue :type Vector%202D%20Structure) (ElapsedSeconds :type Float%20%28double-precision%29) (TriggeredSeconds :type Float%20%28double-precision%29) (InputAction :type Input%20Action%20Object%20Reference :default "/Game/Snake/Blueprints/Input/Action/IA_SnakeMove.IA_SnakeMove"))
  (:Started
    (CallFunction|SnakeMove ActionValue)))

(event EventBeginPlay
  (Utilities|FlowControl|Sequence
    (:then_0
      (bind _asplayer_controller (Utilities|Casting|CastToPlayerController (Pawn|GetController)))
      (Input|AddMappingContext (PlayerController|LocalPlayerSubsystems|GetEnhancedInputLocalPlayerSubsystem _asplayer_controller) "/Game/Snake/Blueprints/Input/IMC_SnakeInputMap.IMC_SnakeInputMap" 0 "(bIgnoreAllPressedKeysUntilRelease=True,bForceImmediately=False,bNotifyUserSettings=False)"))
    (:then_1
      (Variables|SnakeSetting|SetStep 2e+01))
    (:then_2
      (bind _returnvalue (Actor|GetActorOfClass "/Script/FeaturCollection.SnakeTrack"))
      (Variables|Default|SetSnakeTrack _returnvalue))))

(event EventTick
  (params (DeltaSeconds :type Float%20%28single-precision%29))
  (bind _returnvalue (Transformation|GetActorLocation))
  (bind _currentdirect (Variables|SnakeSetting|GetCurrentDirect))
  (bind _step (Variables|SnakeSetting|GetStep))
  (bind _snaketrack (Variables|Default|GetSnakeTrack))
  (bind _returnvalue_2 (* _currentdirect _step))
  (bind _returnvalue_3 (+ _returnvalue _returnvalue_2))
  (Utilities|FlowControl|Delay 0.2)
  (Transformation|SetActorLocation _returnvalue_3 false false)
  (Class|SnakeTrack|SnakeTrackUpdate (Variables|Default|GetSnakeTrack) _returnvalue_3)
  (if (not (Utilities|Array|IsEmpty (Variables|/Script/FeaturCollection.SnakeTrack|GetSnakeBodyActor _snaketrack)))
    (Class|SnakeTrack|SnakeBodyUpdate _snaketrack)))

(fn ConstructionScript)

(fn SnakeMove
  (params (Action :type Vector%202D%20Structure))
  (bind _returnvalue (Transformation|GetActorLocation))
  (bind _step (Variables|SnakeSetting|GetStep))
  (bind _returnvalue_2 (* Action _step))
  (bind _returnvalue_3 (+ _returnvalue _returnvalue_2))
  (Variables|SnakeSetting|SetCurrentDirect Action)
  (Transformation|SetActorLocation _returnvalue_3 false false)
  (Class|SnakeTrack|SnakeTrackUpdate (Variables|Default|GetSnakeTrack) _returnvalue_3))