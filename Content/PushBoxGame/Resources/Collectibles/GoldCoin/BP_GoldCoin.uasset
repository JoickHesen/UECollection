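; BP_GoldCoin is a gold coin collectible that flies to the player on pickup and then disappears.
; On actor overlap it saves its location and, if the other actor is player pawn 0, plays GoldCoinTimeLine.
; The timeline's alpha lerps the coin from that saved location toward the pawn's live position, so it tracks a moving player.
; The coin destroys itself when the timeline finishes, with no score or inventory update here.
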(event Collision|EventActorBeginOverlap
  (params (OtherActor :type Actor%20Object%20Reference))
  (bind _returnvalue (Game|Player|GetPlayerPawn 0))
  ;[1 1 1] 有物体进入触发器范围内调用
  (Variables|Default|SetGoldCoinPosition (Transformation|GetActorLocation))
  (if (== OtherActor _returnvalue)
    (bind _locationalpha (Timeline|GoldCoinTimeLine Play)
      (:Update
        (Transformation|SetActorLocation (Math|Vector|Lerp(Vector) (Variables|Default|GetGoldCoinPosition) (Transformation|GetActorLocation _returnvalue) _locationalpha) false false))
      (:Finished
        (Actor|DestroyActor)))))

(fn ConstructionScript)