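; Blueprint function library for the PushBox game, providing shared helpers for directional hit checks and level loading.
; HitTest line-traces 90 units from an actor along the input direction, draws it for one frame, and returns the hit result and actor.
; ReloadLevel opens the given level, then sets BP_MyPlayerController to Game and UI input with a visible mouse cursor.
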(fn HitTest
  (params (Target :type Actor%20Object%20Reference) (Action%20Value :type Vector%202D%20Structure))
  (bind _returnvalue (Transformation|GetActorLocation Target))
  (bind (_outhit _returnvalue_2) (Collision|LineTraceByChannel Target _returnvalue (+ _returnvalue (* Action%20Value "(X=90.000000,Y=90.000000)")) "TraceTypeQuery3" false 0 "ForOneFrame"))
  (return (.HitActor (Collision|BreakHitResult _outhit)) _returnvalue_2))

(fn ReloadLevel
  (params (Level :type World%20Soft%20Object%20Reference))
  (Game|OpenLevel(byObjectReference) 0 Level)
  (bind _asbp_my_player_controller (Utilities|Casting|CastToBP_MyPlayerController (Game|GetPlayerController 0)))
  (Input|SetInputModeGameandUI _asbp_my_player_controller 0 "DoNotLock" true false)
  (Variables|/Script/Engine.PlayerController|SetbShowMouseCursor _asbp_my_player_controller true))