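; BP_PushBoxGameMode is the game mode for a box-pushing puzzle, deciding when the game is won or lost.
; BeginPlay caches every BP_Box and the player's BP_Player pawn.
; Until the game is over, Tick polls GameSuccess for all boxes having IsTarget set, then checks whether the player's StepNum has run out.
; Either outcome latches GameOver and passes win or loss to BP_MyPlayerController via SetGameState, with winning taking priority.
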(event EventBeginPlay
  (bind _outactors (Actor|GetAllActorsOfClass "/Game/PushBoxGame/Blueprints/Environments/BP_Box.BP_Box_C"))
  (Variables|Default|SetBoxActors _outactors)
  (bind _asbp_player (Utilities|Casting|CastToBP_Player (Game|Player|GetPlayerPawn 0)))
  (Variables|Default|SetMyPlayer _asbp_player))

(event EventTick
  (params (DeltaSeconds :type Float%20%28single-precision%29))
  (bind _returnvalue (Game|GetPlayerController 0))
  (if (not (Variables|Default|GetGameOver))
    (if (CallFunction|GameSuccess)
      (Variables|Default|SetGameOver true)
      (bind _asbp_my_player_controller (Utilities|Casting|CastToBP_MyPlayerController _returnvalue))
      (Default|SetGameState _asbp_my_player_controller true)
      (elif (<= (Variables|/Game/PushBoxGame/Blueprints/Characters/BP_Player.BP_Player_C|GetStepNum (Variables|Default|GetMyPlayer)) 0)
        (Variables|Default|SetGameOver true)
        (bind _asbp_my_player_controller_2 (Utilities|Casting|CastToBP_MyPlayerController _returnvalue))
        (Default|SetGameState _asbp_my_player_controller_2 false)))))

(fn ConstructionScript)

(fn GameSuccess
  (LocalVariables|SetisEnd true)
  (for _array_element (Variables|Default|GetBoxActors)
    (if (not (Variables|/Game/PushBoxGame/Blueprints/Environments/BP_Box.BP_Box_C|GetisTarget _array_element))
      (LocalVariables|SetisEnd false)))
  (return (LocalVariables|GetisEnd)))