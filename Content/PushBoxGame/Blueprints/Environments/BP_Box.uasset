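; BP_Box is a pushable box in a push-box puzzle game that tracks whether it rests on a target.
; Move uses HitTest to check the input direction and, if clear, jumps the box one 100-unit step without sweeping and returns true.
; BoxCollision overlaps with BP_Target set IsTarget and switch the cube's dynamic material Color between yellow on target and light blue off it.
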(event OnComponentBeginOverlap(BoxCollision)
  (params (OverlappedComponent :type Primitive%20Component%20Object%20Reference) (OtherActor :type Actor%20Object%20Reference) (OtherComp :type Primitive%20Component%20Object%20Reference) (OtherBodyIndex :type Integer) (bFromSweep :type Boolean) (SweepResult :type Hit%20Result%20Structure%20%28by%20ref%29))
  (Utilities|Casting|CastToBP_Target OtherActor)
  (Rendering|Material|SetVectorParameterValue (Variables|Default|GetCubeMaterial) "Color" "(R=1.000000,G=0.973712,B=0.000000,A=1.000000)" :!class /Script/Engine.MaterialInstanceDynamic)
  (Variables|Default|SetisTarget true))

(event OnComponentEndOverlap(BoxCollision)
  (params (OverlappedComponent :type Primitive%20Component%20Object%20Reference) (OtherActor :type Actor%20Object%20Reference) (OtherComp :type Primitive%20Component%20Object%20Reference) (OtherBodyIndex :type Integer))
  (Utilities|Casting|CastToBP_Target OtherActor)
  (Rendering|Material|SetVectorParameterValue (Variables|Default|GetCubeMaterial) "Color" "(R=0.200000,G=0.792157,B=1.000000,A=1.000000)" :!class /Script/Engine.MaterialInstanceDynamic)
  (Variables|Default|SetisTarget false))

(event EventBeginPlay
  (bind _returnvalue (Rendering|Material|CreateDynamicMaterialInstance (Variables|Default|GetCube) 0 0 "None" :!class /Script/Engine.PrimitiveComponent))
  (Variables|Default|SetCubeMaterial _returnvalue))

(fn ConstructionScript)

(fn Move
  (params (Action%20Value :type Vector%202D%20Structure))
  (bind _returnvalue (CallFunction|HitTest self Action%20Value))
  (if (not _returnvalue)
    (Transformation|SetActorLocation (+ (Transformation|GetActorLocation) (* Action%20Value "(X=100.000000,Y=100.000000)")) false false)
    (return true)))