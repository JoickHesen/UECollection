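; Player controller for the push-box game that serves both the main play level and the scene editor level.
; BeginPlay creates the matching widget and input mapping by level name, and possession blends the view to BP_Camera.
; In the editor, Tick snaps a selector to a 100-unit grid under the cursor, clicks spawn the chosen type via BP_SceneEditorManager, and Tab toggles menu and selector.
; SetGameState shows the win/lose result and switches to UI-only input.
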(event Input|EnhancedActionEvents|EnhancedInputActionIA_MouseEvent
  (params (ActionValue :type Boolean) (ElapsedSeconds :type Float%20%28double-precision%29) (TriggeredSeconds :type Float%20%28double-precision%29) (InputAction :type Input%20Action%20Object%20Reference :default "/Game/PushBoxGame/Blueprints/Input/Actions/IA_MouseEvent.IA_MouseEvent"))
  (bind _scenemanageractor (Variables|Default|GetSceneManagerActor))
  ;[1 1 1] 鼠标点击输入
  (:Started
    (Utilities|IsValid _scenemanageractor
      (:Is%20Valid
        (Default|CreateActorType _scenemanageractor (Variables|/Game/PushBoxGame/Blueprints/UMG/WBP_EditScene.WBP_EditScene_C|GetSpawnType (Variables|Default|GetEditSceneWidget)))))))

(event EventTick
  (params (DeltaSeconds :type Float%20%28single-precision%29))
  (bind _hightlightactor (Variables|Default|GetHightLightActor))
  ;[1 1 1] 高亮物体检测
  (Utilities|IsValid _hightlightactor
    (:Is%20Valid
      (bind _worldloaction (CallFunction|MouseLocationTranslate))
      (Transformation|SetActorLocation _hightlightactor (Math|Vector|MakeVector (.x _worldloaction) (.y _worldloaction) (.z _worldloaction)) false false))))

(event EventPossess
  (params (PossessedPawn :type Pawn%20Object%20Reference))
  (|CallParentFunction PossessedPawn)
  (Utilities|FlowControl|Delay 0.1)
  (bind _returnvalue (Actor|GetActorOfClass "/Game/PushBoxGame/Blueprints/Characters/BP_Camera.BP_Camera_C"))
  (Game|Player|SetViewTargetwithBlend _returnvalue 0.0 "VTBlend_Linear" 0.0 false))

(event EventBeginPlay
  (bind _returnvalue (Game|GetCurrentLevelName true))
  (switch string _returnvalue
    (:PushBoxMainLevel
      (bind _returnvalue_2 (UserInterface|CreateWidget "/Game/PushBoxGame/Blueprints/UMG/WBP_Main.WBP_Main_C"))
      (bind _output_get (Variables|Default|SetMainWidget _returnvalue_2))
      (UserInterface|Viewport|AddtoViewport _output_get 0))
    (:EditSceneLevel
      (bind _returnvalue_3 (UserInterface|CreateWidget "/Game/PushBoxGame/Blueprints/UMG/WBP_EditScene.WBP_EditScene_C"))
      (bind _output_get_2 (Variables|Default|SetEditSceneWidget _returnvalue_3))
      (UserInterface|Viewport|AddtoViewport _output_get_2 0)
      (bind _returnvalue_4 (Actor|GetActorOfClass "/Game/PushBoxGame/Blueprints/Environments/BP_Selector.BP_Selector_C"))
      (bind _output_get_3 (Variables|Default|SetHightLightActor _returnvalue_4))
      (Rendering|SetActorHiddenInGame _output_get_3 (Variables|Default|GetbHightLightActorVisible))
      (bind _returnvalue_5 (Actor|GetActorOfClass "/Game/PushBoxGame/Blueprints/Controller/BP_SceneEditorManager.BP_SceneEditorManager_C"))
      (Variables|Default|SetSceneManagerActor _returnvalue_5)))
  (Input|AddMappingContext (PlayerController|LocalPlayerSubsystems|GetEnhancedInputLocalPlayerSubsystem self) "/Game/PushBoxGame/Blueprints/Input/IMC_MyInputMap.IMC_MyInputMap" 0 "(bIgnoreAllPressedKeysUntilRelease=True,bForceImmediately=False,bNotifyUserSettings=False)"))

(event Input|KeyboardEvents|Tab
  (params (Key :type Key%20Structure))
  (bind _editscenewidget (Variables|Default|GetEditSceneWidget))
  ;[1 1 1] 控制编辑菜单
  (:Pressed
    (Utilities|IsValid _editscenewidget
      (:Is%20Valid
        (bind _output_get (Variables|Default|SetbSceneWidgetVisible (not (Variables|Default|GetbSceneWidgetVisible))))
        (if _output_get
          (Variables|Default|SetEEditSceneWidgetVisible "Visible")
          (else
            (Variables|Default|SetEEditSceneWidgetVisible "Hidden")))
        (Widget|SetVisibility _editscenewidget (Variables|Default|GetEEditSceneWidgetVisible))
        (bind _output_get_2 (Variables|Default|SetbHightLightActorVisible (not (Variables|Default|GetbHightLightActorVisible))))
        (Rendering|SetActorHiddenInGame (Variables|Default|GetHightLightActor) _output_get_2))
      (:Is%20Not%20Valid
        _))
    (Variables|Default|SetbShowMouseCursor (Variables|Default|GetbSceneWidgetVisible))))

(fn ConstructionScript)

(fn SetGameState
  (params (isWin :type Boolean))
  (Default|ShowGameState (Variables|Default|GetMainWidget) isWin)
  (Input|SetInputModeUIOnly self 0 "DoNotLock" false)
  (Variables|Default|SetbShowMouseCursor true))

(fn MouseLocationTranslate
  (bind _self self)
  (bind (_locationx _locationy) (Game|Player|GetMousePosition _self))
  (bind (_worldposition _worlddirection) (Class|GameplayStatics|DeprojectScreentoWorld _self (Math|Vector2D|MakeVector2D _locationx _locationy)))
  (bind _outhit (Collision|LineTraceByChannel _worldposition (+ _worldposition (* _worlddirection 1e+05)) "TraceTypeQuery4" false 0 "ForOneFrame"))
  (bind _gridlocation (CallFunction|PositionTranslatetoGrid (.Location (Collision|BreakHitResult _outhit))))
  (return _gridlocation))

(fn PositionTranslatetoGrid
  (params (WorldLocation :type Vector))
  (bind _returnvalue (- WorldLocation 5e+01))
  (bind _returnvalue_2 (/ _returnvalue 1e+02))
  (bind _returnvalue_3 (Math|Float|Round (.x _returnvalue_2)))
  (bind _returnvalue_4 (Math|Float|Round (.y _returnvalue_2)))
  (bind _returnvalue_5 (Math|Float|Round (.z _returnvalue_2)))
  (bind _returnvalue_6 (Math|Conversions|ToFloat(Integer) _returnvalue_3))
  (bind _returnvalue_7 (Math|Conversions|ToFloat(Integer) _returnvalue_4))
  (bind _returnvalue_8 (Math|Conversions|ToFloat(Integer) _returnvalue_5))
  (bind _returnvalue_9 (Math|Vector|MakeVector _returnvalue_6 _returnvalue_7 _returnvalue_8))
  (bind _returnvalue_10 (* _returnvalue_9 1e+02))
  (bind _returnvalue_11 (+ _returnvalue_10 5e+01))
  (return (Math|Vector|MakeVector (.x _returnvalue_11) (.y _returnvalue_11) (Math|Float|Max(Float) (.z _returnvalue_11) 5e+01))))