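; BP_Player is the player character of a grid-based box-pushing puzzle game.
; BeginPlay adds the Enhanced Input mapping context and sets a 30-step counter.
; Each move press runs HitTest: empty cells and BP_Target allow the move, BP_Box must first move successfully, and anything else blocks.
; A successful move decrements the counter and jumps the player 100 units per input axis without sweeping.
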(event Input|EnhancedActionEvents|EnhancedInputActionIA_MyMove
  (params (ActionValue :type Vector%202D%20Structure) (ElapsedSeconds :type Float%20%28double-precision%29) (TriggeredSeconds :type Float%20%28double-precision%29) (InputAction :type Input%20Action%20Object%20Reference :default "/Game/PushBoxGame/Blueprints/Input/Actions/IA_MyMove.IA_MyMove"))
  (:Started
    (CallFunction|Move ActionValue)))

(event EventBeginPlay
  (Utilities|FlowControl|Sequence
    (:then_0
      ;[1 1 1] 添加输入映射上下文
      (bind _asplayer_controller (Utilities|Casting|CastToPlayerController (Pawn|GetController)))
      (Input|AddMappingContext (PlayerController|LocalPlayerSubsystems|GetEnhancedInputLocalPlayerSubsystem _asplayer_controller) "/Game/PushBoxGame/Blueprints/Input/IMC_MyInputMap.IMC_MyInputMap" 0 "(bIgnoreAllPressedKeysUntilRelease=True,bForceImmediately=False,bNotifyUserSettings=False)"))
    (:then_1
      (Variables|Default|SetStepNum 30))))

(fn ConstructionScript)

(fn Move
  (params (Action%20Value :type Vector%202D%20Structure))
  (bind (_hitactor _returnvalue) (CallFunction|HitTest self Action%20Value))
  (if _returnvalue
    (bind _asbp_box (Utilities|Casting|CastToBP_Box _hitactor)
      (:then
        (bind _returnvalue_2 (Default|Move _asbp_box Action%20Value))
        (if _returnvalue_2
          (bind _result (Math|Integer|DecrementInt (Variables|Default|GetStepNum) :!label _label)
            (:%20%20
              (Variables|Default|SetStepNum _result)
              (Transformation|SetActorLocation (+ (Transformation|GetActorLocation) (* Action%20Value "(X=100.000000,Y=100.000000)")) false false)))))
      (:CastFailed
        (Utilities|Casting|CastToBP_Target _hitactor)
        (goto _label)))
    (else
      (goto _label))))